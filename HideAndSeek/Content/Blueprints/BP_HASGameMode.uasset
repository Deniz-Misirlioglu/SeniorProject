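; BP_HASGameMode is a game mode Blueprint that maintains a list of the connected player controllers in AllPCs.
; PostLogin calls the parent, adds the new controller and prints a debug message, while OnSwapPlayerControllers also adds the new controller without removing an old one.
; OnLogout removes the exiting controller only if it casts to BP_PC_HAS.
; An unconnected loop for printing controller names never runs.
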(event EventPostLogin
  (params (NewPlayer :type Player%20Controller%20Object%20Reference))
  (|CallParentFunction NewPlayer)
  (Utilities|Array|Add (Variables|Default|GetAll_PCs) NewPlayer)
  (Development|PrintString "OnPostLogin event triggered"))

(event EventOnSwapPlayerControllers
  (params (OldPC :type Player%20Controller%20Object%20Reference) (NewPC :type Player%20Controller%20Object%20Reference))
  (Utilities|Array|Add (Variables|Default|GetAll_PCs) NewPC))

(event EventOnLogout
  (params (ExitingController :type Controller%20Object%20Reference))
  (bind _asbp_pc_has (Utilities|Casting|CastToBP_PC_HAS ExitingController))
  (Utilities|Array|RemoveItem (Variables|Default|GetAll_PCs) _asbp_pc_has))

(fn ConstructionScript)